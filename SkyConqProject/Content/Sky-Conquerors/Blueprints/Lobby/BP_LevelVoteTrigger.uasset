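; BP_LevelVoteTrigger is a lobby trigger that counts votes for a level by how many actors stand inside it.
; Actors beginning overlap add a vote and actors ending overlap remove one, without filtering by actor type.
; Tick writes the current total to a votes text every frame, and the construction script sets the level name text from the LevelName variable.
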(event Collision|EventActorBeginOverlap
  (params (OtherActor :type Actor%20Object%20Reference))
  (Variables|Default|SetTotalVotes (+ (Variables|Default|GetTotalVotes) 1)))

(event EventTick
  (params (DeltaSeconds :type Float%20%28single-precision%29))
  (Rendering|Components|TextRender|SetText (Variables|Default|GetLevelVotesText) (Utilities|Text|ToText(Integer) (Variables|Default|GetTotalVotes))))

(event Collision|EventActorEndOverlap
  (params (OtherActor :type Actor%20Object%20Reference))
  (Variables|Default|SetTotalVotes (- (Variables|Default|GetTotalVotes) 1)))

(fn ConstructionScript
  (Rendering|Components|TextRender|SetText (Variables|Default|GetLevelNameText) (Variables|Default|GetLevelName)))