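; Multiplayer lobby handler that runs the countdown and tallies map votes.
; The authority decrements Timer on Tick, and its OnRep updates MP_Lobby widgets, running SelectLevel's result as a console command at zero.
; AddVote increments VoteArray, which RefreshLevelVotes copies to MP_MapButton widgets, though its call here is unwired.
; SelectLevel looks unfinished: its node building a ServerTravel string for the top-voted level is unused.
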(event Custom|Event%20AddVote
  (params (index :type Integer))
  (bind _votearray (Variables|Default|GetVoteArray))
  (Utilities|Array|SetArrayElem _votearray index (+ (Utilities|Array|Get(acopy) _votearray index) 1)))

(event EventTick
  (params (DeltaSeconds :type Float%20%28single-precision%29))
  (Networking|SwitchHasAuthority
    (:Authority
      (Variables|Default|SetTimer (- (Variables|Default|GetTimer) DeltaSeconds)))))

(fn ConstructionScript)

(fn OnRepTimer
  (bind _foundwidgets (Widget|GetAllWidgetsOfClass "/Game/Sky-Conquerors/Blueprints/Lobby/MP_Lobby.MP_Lobby_C" false))
  (for _array_element _foundwidgets
    (Default|EventUpdateTimer _array_element)
    (if (<= (Variables|Default|GetTimer) 0.0)
      (Development|ExecuteConsoleCommand (|SelectLevel)))))