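; BP_3DLobbyTimer is a lobby countdown that moves the game to the most-voted map when it expires.
; BeginPlay starts a fixed timer, and Tick writes the whole seconds remaining to the Timer text.
; When time runs out, ChangeLevel, on authority only, gathers level names and vote totals from all BP_LevelVoteTrigger actors.
; It server travels to the highest-voted level and prints whether travel succeeded.
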(event EventBeginPlay
  ;[1 1 1] A timer that starts as soon as it is created
  (bind _returnvalue (Utilities|Time|SetTimerbyFunctionName 0 "ChangeLevel" 1e+01)))

(event EventTick
  (params (DeltaSeconds :type Float%20%28single-precision%29))
  ;[1 1 1] A timer that starts as soon as it is created
  (Rendering|Components|TextRender|SetText (Variables|Default|GetTimer) (Utilities|Text|ToText(Integer) (Math|Float|Truncate (Utilities|Time|GetTimerRemainingTimebyHandle (stale EventBeginPlay _returnvalue))))))

(fn ConstructionScript)

(fn ChangeLevel
  ;[1 1 1] Start map with most votes
  (Networking|SwitchHasAuthority
    (:Authority
      (bind _outactors (Actor|GetAllActorsOfClass "/Game/Sky-Conquerors/Blueprints/Lobby/BP_LevelVoteTrigger.BP_LevelVoteTrigger_C"))
      (for _array_element _outactors
        (Utilities|Array|Add (LocalVariables|GetLevelNameArray) (Variables|/Game/Sky-Conquerors/Blueprints/Lobby/BP_LevelVoteTrigger.BP_LevelVoteTrigger_C|GetLevelName _array_element))
        (Utilities|Array|Add (LocalVariables|GetVoteArray) (Variables|/Game/Sky-Conquerors/Blueprints/Lobby/BP_LevelVoteTrigger.BP_LevelVoteTrigger_C|GetTotalVotes _array_element)))
      (Class|HoggeBlueprintLibrary|ServerTravel self (Utilities|String|ToString(Text) (Utilities|Array|Get(acopy) (LocalVariables|GetLevelNameArray) (.IndexOfMaxValue (Math|Integer|MaxOfIntArray (LocalVariables|GetVoteArray))))) false false
        (:CouldServerTravel
          (Development|PrintString "Server Travel worked!" true true "(R=1.000000,G=0.005208,B=0.873558,A=1.000000)" 1e+01))
        (:CouldNotServerTravel
          (Development|PrintString "Server Travel Failed!" true true "(R=1.000000,G=0.005208,B=0.873558,A=1.000000)" 1e+01))))))