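; SB_GameInstance is the Sky-Conquerors game instance, handling session joining and engine connection error events.
; JoinToSelectedServer joins a given session search result with player controller 0 and prints success or failure.
; HandleTravelError switches on the failure type to print a readable debug message for each travel error.
; HandleNetworkError switches on its failure type, but none of its cases perform any action.
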(event Custom|JoinToSelectedServer
  (params (SearchResult :type Blueprint%20Session%20Result%20Structure%20%28by%20ref%29))
  (|JoinSession (Game|GetPlayerController 0) SearchResult
    (:OnSuccess
      (Development|PrintString "SB_GameInstance: Join Success" true true "(R=0.000000,G=1.000000,B=0.000000,A=1.000000)" 15.0))
    (:OnFailure
      (Development|PrintString "SB_GameInstance: Join Failure" true true "(R=1.000000,G=0.000000,B=0.000000,A=1.000000)" 15.0))))

(event EventHandleTravelError
  (params (FailureType :type ETravelFailure%20Enum :default "NoLevel"))
  ;[1 1 1] Travel Error Printing
  (switch Utilities|FlowControl|Switch|SwitchonETravelFailure FailureType
    (:NoLevel
      (Development|PrintString "Travel Error: No level found in the loaded package" true true "(R=1.000000,G=1.000000,B=1.000000,A=1.000000)" 2e+01))
    (:LoadMapFailure
      (Development|PrintString "Travel Error: LoadMap failed on travel (about to Browse to default map)" true true "(R=1.000000,G=1.000000,B=1.000000,A=1.000000)" 2e+01))
    (:InvalidURL
      (Development|PrintString "Travel Error: Invalid URL specified" true true "(R=1.000000,G=1.000000,B=1.000000,A=1.000000)" 2e+01))
    (:PackageMissing
      (Development|PrintString "Travel Error: A package is missing on the client" true true "(R=1.000000,G=1.000000,B=1.000000,A=1.000000)" 2e+01))
    (:PackageVersion
      (Development|PrintString "Travel Error: A package version mismatch has occurred between client and server" true true "(R=1.000000,G=1.000000,B=1.000000,A=1.000000)" 2e+01))
    (:NoDownload
      (Development|PrintString "Travel Error: A package is missing and the client is unable to download the file" true true "(R=1.000000,G=1.000000,B=1.000000,A=1.000000)" 2e+01))
    (:TravelFailure
      (Development|PrintString "Travel Error: General travel failure" true true "(R=1.000000,G=1.000000,B=1.000000,A=1.000000)" 2e+01))
    (:CheatCommands
      (Development|PrintString "Travel Error: Cheat commands have been used disabling travel" true true "(R=1.000000,G=1.000000,B=1.000000,A=1.000000)" 2e+01))
    (:PendingNetGameCreateFailure
      (Development|PrintString "Travel Error: Failed to create the pending net game for travel" true true "(R=1.000000,G=1.000000,B=1.000000,A=1.000000)" 2e+01))
    (:CloudSaveFailure
      (Development|PrintString "Travel Error: Failed to save before travel" true true "(R=1.000000,G=1.000000,B=1.000000,A=1.000000)" 2e+01))
    (:ServerTravelFailure
      (Development|PrintString "Travel Error: There was an error during a server travel to a new map" true true "(R=1.000000,G=1.000000,B=1.000000,A=1.000000)" 2e+01))
    (:ClientTravelFailure
      (Development|PrintString "Travel Error: There was an error during a client travel to a new map" true true "(R=1.000000,G=1.000000,B=1.000000,A=1.000000)" 2e+01))))

(event EventHandleNetworkError
  (params (FailureType :type ENetworkFailure%20Enum :default "NetDriverAlreadyExists") (bIsServer :type Boolean))
  (switch Utilities|FlowControl|Switch|SwitchonENetworkFailure FailureType))