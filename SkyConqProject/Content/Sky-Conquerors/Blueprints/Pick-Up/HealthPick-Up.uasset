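; Health pickup actor that restores a small fixed amount of health to an overlapping actor with a StatsComponent.
; On overlap, while visible, it heals only living targets below MaxHealth and clamps the result to that maximum.
; It then hides itself for a short delay before reappearing, using the Hidden flag to block pickups while respawning rather than destroying the actor.
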(event Collision|EventActorBeginOverlap
  (params (OtherActor :type Actor%20Object%20Reference))
  (bind _returnvalue (Actor|GetComponentbyClass OtherActor "/Game/ThirdPersonBP/Stats-Component.Stats-Component_C"))
  (bind _maxhealth (Variables|/Game/ThirdPersonBP/Stats-Component.Stats-Component_C|GetMaxHealth _returnvalue))
  (if (not (Variables|Rendering|GetbHidden))
    (Math|Float|CompareFloat (Variables|/Game/ThirdPersonBP/Stats-Component.Stats-Component_C|GetCurrentHealth _returnvalue) _maxhealth
      (:<
        (Math|Float|CompareFloat (Variables|/Game/ThirdPersonBP/Stats-Component.Stats-Component_C|GetCurrentHealth _returnvalue) 0.0
          (:>
            (Variables|/Game/ThirdPersonBP/Stats-Component.Stats-Component_C|SetCurrentHealth _returnvalue (Math|Float|Clamp(Float) (+ (Variables|/Game/ThirdPersonBP/Stats-Component.Stats-Component_C|GetCurrentHealth _returnvalue) 0.5) 0.0 _maxhealth))
            (Rendering|SetActorHiddenInGame true)
            (Utilities|FlowControl|Delay 3.0)
            (Rendering|SetActorHiddenInGame false)))))))

(fn ConstructionScript)